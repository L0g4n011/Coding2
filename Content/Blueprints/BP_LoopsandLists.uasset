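; BP_LoopsandLists is a demo actor that exercises array shuffling and looping through on-screen debug prints.
; BeginPlay starts SimpleDelayLoop, a custom event that counts each pass, waits one second, calls PrintColors, then calls itself to repeat endlessly.
; PrintColors shuffles the TextColors array and prints each element's index in that color, followed by a completion message.
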(event `Print Colors`
  (bind _textcolors (`self.TextColors`))
  (`KismetArrayLibrary.Array_Shuffle` _textcolors)
  (for (_array_element _array_index) _textcolors
    (`KismetSystemLibrary.PrintString` (`KismetStringLibrary.Concat_StrStr` "Printing color # " (`KismetStringLibrary.Conv_IntToString` _array_index)) true true _array_element))
  (`KismetSystemLibrary.PrintString` "Done Printing Colors" true true (struct :`A` 1.0)))

(event `SimpleDelayLoop`
  (`KismetSystemLibrary.PrintString` (`KismetStringLibrary.Concat_StrStr` "Starting Delay Loop# " (`KismetStringLibrary.Conv_IntToString` (`self.DelayLoopCount`))))
  (`/Engine/EditorBlueprintResources/StandardMacros.IncrementInt` (`self.DelayLoopCount`)
    (:`  `
      (`KismetSystemLibrary.Delay` 1.0)
      (`self.Print Colors`)
      (`self.SimpleDelayLoop`))))

(event `self.ReceiveBeginPlay`
  (`KismetSystemLibrary.PrintString` "Loops and Lists are active")
  (`self.SimpleDelayLoop`))

(fn `UserConstructionScript`)